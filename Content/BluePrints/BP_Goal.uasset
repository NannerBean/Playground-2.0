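; BP_Goal is the sheep pen goal that counts herded sheep and triggers the win.
; A GoalTrigger overlap prints a debug message, then casts to BP_Sheep, flags it as in the pen and increments SheepCounter without checking for repeat entries.
; When the incremented count reaches ten (tested as counter + 1 == 11), it shows WBP_YouWin, plays its Cowboy animation and a yeehaw sound.
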(event OnComponentBeginOverlap(GoalTrigger)
  (params (OverlappedComponent :type Primitive%20Component%20Object%20Reference) (OtherActor :type Actor%20Object%20Reference) (OtherComp :type Primitive%20Component%20Object%20Reference) (OtherBodyIndex :type Integer) (bFromSweep :type Boolean) (SweepResult :type Hit%20Result%20Structure%20%28by%20ref%29))
  (Development|PrintString "Got Sheep!" true true "(R=1.000000,G=0.005688,B=0.000000,A=1.000000)")
  (bind _asbp_sheep (Utilities|Casting|CastToBP_Sheep OtherActor))
  (bind _output_get (Variables|Default|SetSheep _asbp_sheep))
  (Variables|/Game/BluePrints/BP_Sheep.BP_Sheep_C|SetbIsInPen _output_get true)
  (Variables|Default|SetSheepCounter (+ (Variables|Default|GetSheepCounter) 1.0))
  (if (== (+ (Variables|Default|GetSheepCounter) 1.0) 11.0)
    (Development|PrintString "You got all sheep !" true true "(R=1.000000,G=0.000000,B=0.021849,A=1.000000)")
    (bind _returnvalue (UserInterface|CreateWidget "/Game/Widgets/WBP_YouWin.WBP_YouWin_C"))
    (bind _output_get_2 (Variables|Default|SetYouWIn _returnvalue))
    (UserInterface|Viewport|AddtoViewport _output_get_2 0)
    (UserInterface|Animation|PlayAnimation _output_get_2 (Variables|/Game/Widgets/WBP_YouWin.WBP_YouWin_C|GetCowboy _output_get_2) 0.0 1 "Forward" 1.0 false)
    (Audio|PlaySound2D "/Game/SFX/102437__shawshank73__scottstoked_yeehaw.102437__shawshank73__scottstoked_yeehaw" 1.0 1.0 0.0 0 0)))

(fn ConstructionScript)