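; BPC_Interact is an interaction component for the first-person character, caching that character's camera on BeginPlay.
; TrytoInteract runs a 300-unit visibility line trace forward from the camera, with a timed debug line.
; On a hit it prints the actor's name and distance, then casts it to BP_Torch and calls LightUnlight on it.
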(event Custom|Try%20to%20Interact
  (bind _first_person_camera (Variables|Default|GetFirst%20Person%20Camera))
  (bind _returnvalue (Transformation|GetWorldLocation _first_person_camera))
  (bind (_outhit _returnvalue_2) (Collision|LineTraceByChannel _returnvalue (+ _returnvalue (* (Math|Vector|GetForwardVector _first_person_camera) 3e+02)) "TraceTypeQuery1" false 0 "ForDuration"))
  (if _returnvalue_2
    (Development|PrintText (Utilities|Text|FormatText "I am touching {name} {distance} away!" (Utilities|GetDisplayName (.HitActor (Collision|BreakHitResult _outhit))) (.Distance (Collision|BreakHitResult _outhit))))
    (bind _asbp_torch (Utilities|Casting|CastToBP_Torch (.HitActor (Collision|BreakHitResult _outhit))))
    (bind _output_get (Variables|Default|SetAs%20BP%20Torch _asbp_torch))
    (Default|Light/Unlight _output_get)))

(event EventBeginPlay
  (bind _asbp_first_person_character (Utilities|Casting|CastToBP_FirstPersonCharacter (Components|GetOwner)))
  (Variables|Default|SetFirst%20Person%20Camera (Variables|/Game/FirstPerson/Blueprints/BP_FirstPersonCharacter.BP_FirstPersonCharacter_C|GetFirstPersonCamera _asbp_first_person_character)))