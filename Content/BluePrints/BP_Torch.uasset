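; BP_Torch is a puzzle torch that toggles lit and unlit, feeding a counter on the level's BP_LargeDoor to open it.
; BeginPlay hides the Niagara fire and finds the door.
; Light/Unlight uses a FlipFlop to toggle flame and sound, adding the torch's Value when lit.
; Unlighting subtracts one if Value is one, otherwise adds one; either toggle opens the door when the counter equals three.
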(event Custom|Light/Unlight
  (bind _ns_fire (Variables|Default|GetNS_Fire))
  (Utilities|FlowControl|FlipFlop
    (:A
      (Variables|Default|SetbIsLit true)
      (Rendering|SetVisibility _ns_fire true false)
      (Audio|PlaySound2D "/Game/SFX/676471__neartheatmoshphere__lighter-short.676471__neartheatmoshphere__lighter-short" 1.0 1.0 0.0 0 0)
      (bind _output_get (Variables|/Game/BluePrints/BP_LargeDoor.BP_LargeDoor_C|Setvalue%20counter (stale EventBeginPlay _output_get) (+ (Variables|Default|GetValue) (Variables|/Game/BluePrints/BP_LargeDoor.BP_LargeDoor_C|Getvalue%20counter (stale EventBeginPlay _output_get)))))
      (Development|PrintText (Utilities|Text|FormatText "Counter is at {value}" _output_get) true true "(R=1.000000,G=0.024158,B=0.000000,A=1.000000)")
      (if (== _output_get 3.0)
        (Default|OpenDoor (stale EventBeginPlay _output_get) :!label _label)))
    (:B
      (Variables|Default|SetbIsLit false)
      (Rendering|SetVisibility _ns_fire false false)
      (Audio|PlaySound2D "/Game/SFX/831929__1bob__flamethrower.831929__1bob__flamethrower" 1.0 1.0 0.0 0 0)
      (if (== (Variables|Default|GetValue) 1.0)
        (bind _output_get_2 (Variables|/Game/BluePrints/BP_LargeDoor.BP_LargeDoor_C|Setvalue%20counter (stale EventBeginPlay _output_get) (- (Variables|/Game/BluePrints/BP_LargeDoor.BP_LargeDoor_C|Getvalue%20counter (stale EventBeginPlay _output_get)) 1.0)))
        (Development|PrintText (Utilities|Text|FormatText "Counter is at {value}" _output_get_2) true true "(R=1.000000,G=0.024158,B=0.000000,A=1.000000)")
        (if (== _output_get_2 3.0)
          (goto _label)
          (else
            (Development|PrintString "Not enough to open")))
        (else
          (bind _output_get_3 (Variables|/Game/BluePrints/BP_LargeDoor.BP_LargeDoor_C|Setvalue%20counter (stale EventBeginPlay _output_get) (+ (Variables|/Game/BluePrints/BP_LargeDoor.BP_LargeDoor_C|Getvalue%20counter (stale EventBeginPlay _output_get)) 1.0)))
          (Development|PrintText (Utilities|Text|FormatText "Counter is at {value}" _output_get_3) true true "(R=1.000000,G=0.000000,B=0.003675,A=1.000000)")
          (if (== _output_get_3 3.0)
            (goto _label)
            (else
              (Development|PrintString "Not enough to open"))))))))

(event EventBeginPlay
  (Rendering|SetVisibility (Variables|Default|GetNS_Fire) false false)
  (bind _returnvalue (Actor|GetActorOfClass "/Game/BluePrints/BP_LargeDoor.BP_LargeDoor_C"))
  (bind _output_get (Variables|Default|SetLargeDoor _returnvalue)))

(fn ConstructionScript)