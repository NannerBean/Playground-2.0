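; BP_Sheep is a herdable sheep that the player pushes around by getting close, until it is in a pen.
; A self-repeating one-second check tests whether the first-person character overlaps its PersonalSpace and stops once IsInPen is set.
; On overlap, the sheep jumps a fixed distance along the player's forward vector, copies the player mesh's rotation and occasionally plays a sheep sound.
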(event Custom|Check%20for%20Player
  (if (not (Variables|Default|GetbIsInPen))
    (Development|PrintString "checking...")
    (bind _returnvalue (Actor|GetActorOfClass "/Game/FirstPerson/Blueprints/BP_FirstPersonCharacter.BP_FirstPersonCharacter_C"))
    (bind _output_get (Variables|Default|SetFirst%20Person%20Character _returnvalue))
    (bind _output_get_2 (Variables|Default|SetPlayerIsNear (Collision|IsOverlappingActor (Variables|Default|GetPersonalSpace) (Components|GetOwner (Variables|/Script/Engine.Character|GetCapsuleComponent _output_get)) :!class /Script/Engine.PrimitiveComponent)))
    (if _output_get_2
      (Transformation|SetWorldTransform (Variables|Default|GetDefaultSceneRoot) (Math|Transform|MakeTransform (+ (Transformation|GetWorldLocation (Variables|Default|GetDefaultSceneRoot)) (* (Math|Vector|GetForwardVector (Variables|/Script/Engine.Character|GetCapsuleComponent _output_get)) 2.5e+02)) (Transformation|GetWorldRotation (Variables|/Game/FirstPerson/Blueprints/BP_FirstPersonCharacter.BP_FirstPersonCharacter_C|GetFirstPersonMesh _output_get)) "1.000000,1.000000,1.000000") false false)
      (if (== (Math|Random|RandomInteger 10) 1)
        (Audio|PlaySound2D "/Game/SFX/SC_Sheep.SC_Sheep" 1.0 1.0 0.0 0 0))
      (Utilities|FlowControl|Delay 1.0)
      (CallFunction|CheckforPlayer)
      (else
        (Utilities|FlowControl|Delay 1.0)
        (CallFunction|CheckforPlayer)))))

(event EventBeginPlay
  (CallFunction|CheckforPlayer))

(fn ConstructionScript)