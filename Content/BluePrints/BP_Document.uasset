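; BP_Document is an actor that opens the WBP_LogicPoem widget when the first-person character overlaps its collision component.
; On overlap, if the character's IsPaused flag is false, it sets the flag and pauses the game.
; It then switches input to UI only, shows the mouse cursor and adds the widget to the viewport, with no unpause logic in this Blueprint.
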(event OnComponentBeginOverlap(Collison)
  (params (OverlappedComponent :type Primitive%20Component%20Object%20Reference) (OtherActor :type Actor%20Object%20Reference) (OtherComp :type Primitive%20Component%20Object%20Reference) (OtherBodyIndex :type Integer) (bFromSweep :type Boolean) (SweepResult :type Hit%20Result%20Structure%20%28by%20ref%29))
  (bind _returnvalue (Game|GetPlayerController 0))
  (bind _asbp_first_person_character (Utilities|Casting|CastToBP_FirstPersonCharacter OtherActor))
  (bind _output_get (Variables|Default|SetFirst%20Person%20Character _asbp_first_person_character))
  (if (not (Variables|/Game/FirstPerson/Blueprints/BP_FirstPersonCharacter.BP_FirstPersonCharacter_C|GetbIsPaused _output_get))
    (bind _output_get_2 (Variables|/Game/FirstPerson/Blueprints/BP_FirstPersonCharacter.BP_FirstPersonCharacter_C|SetbIsPaused _output_get true))
    (Game|SetGamePaused _output_get_2)
    (Input|SetInputModeUIOnly _returnvalue 0 "DoNotLock" false)
    (Variables|/Script/Engine.PlayerController|SetbShowMouseCursor _returnvalue true)
    (bind _returnvalue_2 (UserInterface|CreateWidget "/Game/Widgets/WBP_LogicPoem.WBP_LogicPoem_C"))
    (UserInterface|Viewport|AddtoViewport _returnvalue_2 0)))

(fn ConstructionScript)